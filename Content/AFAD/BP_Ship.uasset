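; Player-driven ship pawn that tows BP_Plastic_Boat through a physics constraint and cable.
; Enhanced Input applies thrust and yaw torque to the hull, while E sphere-traces to send interact messages.
; F swaps the health UI and, when the boat overlaps Box, breaks the tow and possesses it.
; Hard impacts drain health; at zero, buoyancy is removed and the game quits after a delay, or immediately upon overlapping TaklaAtma.
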(event OnComponentBeginOverlap(Box)
  (params (OverlappedComponent :type Primitive%20Component%20Object%20Reference) (OtherActor :type Actor%20Object%20Reference) (OtherComp :type Primitive%20Component%20Object%20Reference) (OtherBodyIndex :type Integer) (bFromSweep :type Boolean) (SweepResult :type Hit%20Result%20Structure%20%28by%20ref%29))
  (bind _asbp_plastic_boat (Utilities|Casting|CastToBP_Plastic_Boat OtherActor))
  (Variables|Default|SetBp_Plastic_Boat _asbp_plastic_boat)
  (Variables|Default|SetCanPossess2 true))

(event OnComponentEndOverlap(Box)
  (params (OverlappedComponent :type Primitive%20Component%20Object%20Reference) (OtherActor :type Actor%20Object%20Reference) (OtherComp :type Primitive%20Component%20Object%20Reference) (OtherBodyIndex :type Integer))
  (bind _asbp_plastic_boat (Utilities|Casting|CastToBP_Plastic_Boat OtherActor))
  (Variables|Default|SetBp_Plastic_Boat _asbp_plastic_boat)
  (Variables|Default|SetCanPossess2 false))

(event OnComponentBeginOverlap(Box1)
  (params (OverlappedComponent :type Primitive%20Component%20Object%20Reference) (OtherActor :type Actor%20Object%20Reference) (OtherComp :type Primitive%20Component%20Object%20Reference) (OtherBodyIndex :type Integer) (bFromSweep :type Boolean) (SweepResult :type Hit%20Result%20Structure%20%28by%20ref%29))
  (bind _astakla_atma (Utilities|Casting|CastToTaklaAtma OtherActor))
  (Variables|Default|SetAs%20Takla%20Atma _astakla_atma)
  (Actor|DestroyActor)
  (Game|QuitGame 0 "Quit" false))

(event OnComponentHit(Ship)
  (params (HitComponent :type Primitive%20Component%20Object%20Reference) (OtherActor :type Actor%20Object%20Reference) (OtherComp :type Primitive%20Component%20Object%20Reference) (NormalImpulse :type Vector :default "0, 0, 0") (Hit :type Hit%20Result%20Structure%20%28by%20ref%29))
  (bind _returnvalue (Math|Vector|VectorLength NormalImpulse))
  (if (> _returnvalue 5e+04)
    (Variables|Default|SetHealth (Math|Float|Clamp(Float) (- (Variables|Default|GetHealth) (/ _returnvalue 1e+04)) 0.0 1e+02))
    (if (== (Variables|Default|GetHealth) 0.0)
      (Components|DestroyComponent (Variables|Default|GetBuoyancy))
      (Utilities|FlowControl|Delay 4.0)
      (Game|QuitGame 0 "Quit" false))))

(event Input|EnhancedActionEvents|EnhancedInputActionIA_Move_Ship
  (params (ActionValue :type Float%20%28double-precision%29) (ElapsedSeconds :type Float%20%28double-precision%29) (TriggeredSeconds :type Float%20%28double-precision%29) (InputAction :type Input%20Action%20Object%20Reference :default "/Game/Input/Actions/IA_Move_Ship.IA_Move_Ship"))
  (Physics|AddForce (Variables|Default|GetShip) (Math|Vector|RotateVector (Math|Vector|MakeVector (* ActionValue 7e+02) 0.0 0.0) (Math|Rotator|CombineRotators (Transformation|GetActorRotation) "0.000000,90.000000,0.000000")) "None" true))

(event Input|EnhancedActionEvents|EnhancedInputActionIA_Steer_Ship
  (params (ActionValue :type Float%20%28double-precision%29) (ElapsedSeconds :type Float%20%28double-precision%29) (TriggeredSeconds :type Float%20%28double-precision%29) (InputAction :type Input%20Action%20Object%20Reference :default "/Game/Input/Actions/IA_Steer_Ship.IA_Steer_Ship"))
  (Class|PrimitiveComponent|AddTorqueinDegrees (Variables|Default|GetShip) (Math|Vector|MakeVector 0.0 0.0 (* ActionValue 6e+01)) "None" true))

(event EventBeginPlay
  (Utilities|FlowControl|Sequence
    (:then_0
      (bind _asgm_afad (Utilities|Casting|CastToGM_Afad (Game|GetGameMode)))
      (Default|ShipHealthVisibility (Variables|/Game/AFAD/GM_Afad.GM_Afad_C|GetCan _asgm_afad)))
    (:then_1
      (Input|AddMappingContext (PlayerController|LocalPlayerSubsystems|GetEnhancedInputLocalPlayerSubsystem (Pawn|GetLocalViewingPlayerController)) "/Game/Input/IMC_Ship.IMC_Ship" 1 "(bIgnoreAllPressedKeysUntilRelease=True,bForceImmediately=False,bNotifyUserSettings=False)")
      (bind _returnvalue (Actor|GetActorOfClass "/Game/AFAD/BP_Plastic_Boat.BP_Plastic_Boat_C"))
      (Variables|Default|SetBp_Plastic_Boat _returnvalue)
      (Class|PhysicsConstraintComponent|SetConstrainedComponents (Variables|Default|GetPhysicsConstraint) (Variables|Default|GetShip) "None" (Variables|/Game/AFAD/BP_Plastic_Boat.BP_Plastic_Boat_C|GetPlastic_Boat (Variables|Default|GetBp_Plastic_Boat)) "None")
      (Class|CableComponent|SetAttachEndtoComponent (Variables|Default|GetCable) (Variables|/Game/AFAD/BP_Plastic_Boat.BP_Plastic_Boat_C|GetPlastic_Boat (Variables|Default|GetBp_Plastic_Boat)) "EndSocket"))))

(event Input|MouseEvents|MouseX
  (params (AxisValue :type Float%20%28single-precision%29))
  (Pawn|Input|AddControllerYawInput AxisValue))

(event Input|MouseEvents|MouseY
  (params (AxisValue :type Float%20%28single-precision%29))
  (Pawn|Input|AddControllerPitchInput (* AxisValue -1.0)))

(event Input|KeyboardEvents|F
  (params (Key :type Key%20Structure :default "None"))
  (:Pressed
    (bind _asgm_afad (Utilities|Casting|CastToGM_Afad (Game|GetGameMode)))
    (Default|ShipHealthHidden (Variables|/Game/AFAD/GM_Afad.GM_Afad_C|GetCan _asgm_afad))
    (Default|BoatHealthVisibility (Variables|/Game/AFAD/GM_Afad.GM_Afad_C|GetCan _asgm_afad))
    (if (Variables|Default|GetCanPossess2)
      (Class|PhysicsConstraintComponent|BreakConstraint (Variables|Default|GetPhysicsConstraint))
      (Rendering|SetVisibility (Variables|Default|GetCable) false false)
      (Pawn|Possess (Game|GetPlayerController 0) (Variables|Default|GetBp_Plastic_Boat))
      (else
        (Development|PrintString "Ship Far")))))

(event Input|KeyboardEvents|E
  (params (Key :type Key%20Structure :default "None"))
  (:Pressed
    (bind _hitactor (Utilities|Interact)
      (:IsValid
        (Class|BPIInteract|Interactable(Message) _hitactor)))))

(fn ConstructionScript)

(fn GetInteractState
  (return false))