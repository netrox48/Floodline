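; BP_İskele is an interactable in the AFAD rescue content that places surviving characters (Jamila, Dave, Kamira, Karen, MRKim) at set transforms.
; Each survival flag gates a DoOnce that either spawns that character marked safe, with physics off and its help component destroyed, or prints that they did not survive.
; Interactable and Interactable1 duplicate this logic with separate DoOnce gates, so each can spawn its own set.
; Both GetInteractState functions return false.
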(event EventInteractable1
  (Utilities|FlowControl|Sequence
    (:then_0
      (if (Variables|Default|GetJamila)
        (Utilities|FlowControl|DoOnce false
          (:Completed
            (bind _returnvalue (Game|SpawnActorfromClass "/Game/AFAD/BP_Jamila.BP_Jamila_C" (Variables|Default|GetSpawn%20Transform) "Undefined" "MultiplyWithRoot" 0 true 0))
            (Physics|SetSimulatePhysics (Variables|/Game/AFAD/BP_Jamila.BP_Jamila_C|GetJamila _returnvalue) false)
            (Components|DestroyComponent (Variables|/Game/AFAD/BP_Jamila.BP_Jamila_C|GetHelpWoman _returnvalue))))
        (else
          (Utilities|FlowControl|DoOnce false
            (:Completed
              (Development|PrintString "Jamila did not survive "))))))
    (:then_1
      (if (Variables|Default|GetDave)
        (Utilities|FlowControl|DoOnce false
          (:Completed
            (bind _returnvalue_2 (Game|SpawnActorfromClass "/Game/AFAD/BP_Dave.BP_Dave_C" (Variables|Default|GetSpawn%20Transform_0) "Undefined" "MultiplyWithRoot" 0 true 0))
            (Physics|SetSimulatePhysics (Variables|/Game/AFAD/BP_Dave.BP_Dave_C|GetDave _returnvalue_2) false)
            (Components|DestroyComponent (Variables|/Game/AFAD/BP_Dave.BP_Dave_C|GetHelpMan _returnvalue_2))))
        (else
          (Utilities|FlowControl|DoOnce false
            (:Completed
              (Development|PrintString "Dave did not survive "))))))
    (:then_2
      (if (Variables|Default|GetKamira)
        (Utilities|FlowControl|DoOnce false
          (:Completed
            (bind _returnvalue_3 (Game|SpawnActorfromClass "/Game/AFAD/BP_Kamira.BP_Kamira_C" (Variables|Default|GetSpawn%20Transform_1) "Undefined" "MultiplyWithRoot" 0 true 0))
            (Physics|SetSimulatePhysics (Variables|/Game/AFAD/BP_Kamira.BP_Kamira_C|GetKamira _returnvalue_3) false)
            (Components|DestroyComponent (Variables|/Game/AFAD/BP_Kamira.BP_Kamira_C|GetHelpWoman _returnvalue_3))))
        (else
          (Utilities|FlowControl|DoOnce false
            (:Completed
              (Development|PrintString "Kamira did not survive "))))))
    (:then_3
      (if (Variables|Default|GetKaren)
        (Utilities|FlowControl|DoOnce false
          (:Completed
            (bind _returnvalue_4 (Game|SpawnActorfromClass "/Game/AFAD/BP_Karen.BP_Karen_C" (Variables|Default|GetSpawn%20Transform_2) "Undefined" "MultiplyWithRoot" 0 true 0))
            (Physics|SetSimulatePhysics (Variables|/Game/AFAD/BP_Karen.BP_Karen_C|GetKaren _returnvalue_4) false)
            (Components|DestroyComponent (Variables|/Game/AFAD/BP_Karen.BP_Karen_C|GetHelpWoman _returnvalue_4))))
        (else
          (Utilities|FlowControl|DoOnce false
            (:Completed
              (Development|PrintString "Karen did not survive "))))))
    (:then_4
      (if (Variables|Default|GetMRKim)
        (Utilities|FlowControl|DoOnce false
          (:Completed
            (bind _returnvalue_5 (Game|SpawnActorfromClass "/Game/AFAD/BP_MRKim.BP_MRKim_C" (Variables|Default|GetSpawn%20Transform_3) "Undefined" "MultiplyWithRoot" 0 true 0))
            (Physics|SetSimulatePhysics (Variables|/Game/AFAD/BP_MRKim.BP_MRKim_C|GetMRKim _returnvalue_5) false)
            (Components|DestroyComponent (Variables|/Game/AFAD/BP_MRKim.BP_MRKim_C|GetHelpMan _returnvalue_5))))
        (else
          (Utilities|FlowControl|DoOnce false
            (:Completed
              (Development|PrintString "MRKim did not survive "))))))))

(event EventInteractable
  (Utilities|FlowControl|Sequence
    (:then_0
      (if (Variables|Default|GetJamila)
        (Utilities|FlowControl|DoOnce false
          (:Completed
            (bind _returnvalue (Game|SpawnActorfromClass "/Game/AFAD/BP_Jamila.BP_Jamila_C" (Variables|Default|GetSpawn%20Transform) "Undefined" "MultiplyWithRoot" 0 true 0))
            (Physics|SetSimulatePhysics (Variables|/Game/AFAD/BP_Jamila.BP_Jamila_C|GetJamila _returnvalue) false)
            (Components|DestroyComponent (Variables|/Game/AFAD/BP_Jamila.BP_Jamila_C|GetHelpWoman _returnvalue))))
        (else
          (Utilities|FlowControl|DoOnce false
            (:Completed
              (Development|PrintString "Jamila did not survive "))))))
    (:then_1
      (if (Variables|Default|GetDave)
        (Utilities|FlowControl|DoOnce false
          (:Completed
            (bind _returnvalue_2 (Game|SpawnActorfromClass "/Game/AFAD/BP_Dave.BP_Dave_C" (Variables|Default|GetSpawn%20Transform_0) "Undefined" "MultiplyWithRoot" 0 true 0))
            (Physics|SetSimulatePhysics (Variables|/Game/AFAD/BP_Dave.BP_Dave_C|GetDave _returnvalue_2) false)
            (Components|DestroyComponent (Variables|/Game/AFAD/BP_Dave.BP_Dave_C|GetHelpMan _returnvalue_2))))
        (else
          (Utilities|FlowControl|DoOnce false
            (:Completed
              (Development|PrintString "Dave did not survive "))))))
    (:then_2
      (if (Variables|Default|GetKamira)
        (Utilities|FlowControl|DoOnce false
          (:Completed
            (bind _returnvalue_3 (Game|SpawnActorfromClass "/Game/AFAD/BP_Kamira.BP_Kamira_C" (Variables|Default|GetSpawn%20Transform_1) "Undefined" "MultiplyWithRoot" 0 true 0))
            (Physics|SetSimulatePhysics (Variables|/Game/AFAD/BP_Kamira.BP_Kamira_C|GetKamira _returnvalue_3) false)
            (Components|DestroyComponent (Variables|/Game/AFAD/BP_Kamira.BP_Kamira_C|GetHelpWoman _returnvalue_3))))
        (else
          (Utilities|FlowControl|DoOnce false
            (:Completed
              (Development|PrintString "Kamira did not survive "))))))
    (:then_3
      (if (Variables|Default|GetKaren)
        (Utilities|FlowControl|DoOnce false
          (:Completed
            (bind _returnvalue_4 (Game|SpawnActorfromClass "/Game/AFAD/BP_Karen.BP_Karen_C" (Variables|Default|GetSpawn%20Transform_2) "Undefined" "MultiplyWithRoot" 0 true 0))
            (Physics|SetSimulatePhysics (Variables|/Game/AFAD/BP_Karen.BP_Karen_C|GetKaren _returnvalue_4) false)
            (Components|DestroyComponent (Variables|/Game/AFAD/BP_Karen.BP_Karen_C|GetHelpWoman _returnvalue_4))))
        (else
          (Utilities|FlowControl|DoOnce false
            (:Completed
              (Development|PrintString "Karen did not survive "))))))
    (:then_4
      (if (Variables|Default|GetMRKim)
        (Utilities|FlowControl|DoOnce false
          (:Completed
            (bind _returnvalue_5 (Game|SpawnActorfromClass "/Game/AFAD/BP_MRKim.BP_MRKim_C" (Variables|Default|GetSpawn%20Transform_3) "Undefined" "MultiplyWithRoot" 0 true 0))
            (Physics|SetSimulatePhysics (Variables|/Game/AFAD/BP_MRKim.BP_MRKim_C|GetMRKim _returnvalue_5) false)
            (Components|DestroyComponent (Variables|/Game/AFAD/BP_MRKim.BP_MRKim_C|GetHelpMan _returnvalue_5))))
        (else
          (Utilities|FlowControl|DoOnce false
            (:Completed
              (Development|PrintString "MRKim did not survive "))))))))

(fn ConstructionScript)

(fn GetInteractState
  (return false))

(fn GetInteractState1
  (return false))