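; BP_Harvester is an alien harvester actor that travels along a route and damages player ships it touches.
; On BeginPlay it finds the BP_ROTA actor, and a Timeline moves it along that actor's spline, matching position and rotation to the distance travelled.
; When its Box overlaps a BP_Ship, it subtracts a fixed amount from the ship's Health and calls Death on it.
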(event OnComponentBeginOverlap(Box)
  (params (OverlappedComponent :type Primitive%20Component%20Object%20Reference) (OtherActor :type Actor%20Object%20Reference) (OtherComp :type Primitive%20Component%20Object%20Reference) (OtherBodyIndex :type Integer) (bFromSweep :type Boolean) (SweepResult :type Hit%20Result%20Structure%20%28by%20ref%29))
  (bind _asbp_ship (Utilities|Casting|CastToBP_Ship OtherActor))
  (bind _output_get (Variables|Default|SetAs%20BP%20Ship _asbp_ship))
  (Variables|/Game/AFAD/BP_Ship.BP_Ship_C|SetHealth _output_get (- (Variables|/Game/AFAD/BP_Ship.BP_Ship_C|GetHealth _output_get) 1e+01))
  (Default|Death _output_get))

(event Collision|EventActorBeginOverlap
  (params (OtherActor :type Actor%20Object%20Reference)))

(event EventTick
  (params (DeltaSeconds :type Float%20%28single-precision%29)))

(event EventBeginPlay
  (bind _returnvalue (Actor|GetActorOfClass "/Game/AFAD/EFE/ALIEN/BP_ROTA.BP_ROTA_C"))
  (bind _newtrack_0 (Timeline|Timeline Play)
    (:Update
      (Transformation|SetActorLocationAndRotation (Spline|GetLocationatDistanceAlongSpline (Variables|/Game/AFAD/EFE/ALIEN/BP_ROTA.BP_ROTA_C|GetSpline _returnvalue) (* _newtrack_0 (Spline|GetSplineLength (Variables|/Game/AFAD/EFE/ALIEN/BP_ROTA.BP_ROTA_C|GetSpline _returnvalue))) "World") (Spline|GetRotationatDistanceAlongSpline (Variables|/Game/AFAD/EFE/ALIEN/BP_ROTA.BP_ROTA_C|GetSpline _returnvalue) (* _newtrack_0 (Spline|GetSplineLength (Variables|/Game/AFAD/EFE/ALIEN/BP_ROTA.BP_ROTA_C|GetSpline _returnvalue))) "World")))))

(fn ConstructionScript)