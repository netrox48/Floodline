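; BP_Plastic_Boat is a player-driven physics boat pawn that works away from BP_Ship, steered with Enhanced Input force and torque.
; F re-docks it when near the ship: teleporting to BoatArea, possessing the ship, constraining the boat and swapping health UI.
; Zero health or touching TaklaAtma forces the same return; a timer, set only at BeginPlay, drains health away from the ship.
; E sphere-traces for interactables and messages them.
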(event OnComponentBeginOverlap(Box)
  (params (OverlappedComponent :type Primitive%20Component%20Object%20Reference) (OtherActor :type Actor%20Object%20Reference) (OtherComp :type Primitive%20Component%20Object%20Reference) (OtherBodyIndex :type Integer) (bFromSweep :type Boolean) (SweepResult :type Hit%20Result%20Structure%20%28by%20ref%29))
  (bind _asbp_ship (Utilities|Casting|CastToBP_Ship OtherActor))
  (Variables|Default|SetBP_Ship _asbp_ship)
  (Variables|Default|SetCanPossess true))

(event OnComponentEndOverlap(Box)
  (params (OverlappedComponent :type Primitive%20Component%20Object%20Reference) (OtherActor :type Actor%20Object%20Reference) (OtherComp :type Primitive%20Component%20Object%20Reference) (OtherBodyIndex :type Integer))
  (bind _asbp_ship (Utilities|Casting|CastToBP_Ship OtherActor))
  (Variables|Default|SetBP_Ship _asbp_ship)
  (Variables|Default|SetCanPossess false))

(event OnComponentBeginOverlap(Box1)
  (params (OverlappedComponent :type Primitive%20Component%20Object%20Reference) (OtherActor :type Actor%20Object%20Reference) (OtherComp :type Primitive%20Component%20Object%20Reference) (OtherBodyIndex :type Integer) (bFromSweep :type Boolean) (SweepResult :type Hit%20Result%20Structure%20%28by%20ref%29))
  (bind _bp_ship (Variables|Default|GetBP_Ship))
  (bind _boat_area (Variables|/Game/AFAD/BP_Ship.BP_Ship_C|GetBoat%20Area _bp_ship))
  (bind _astakla_atma (Utilities|Casting|CastToTaklaAtma OtherActor))
  (Variables|Default|SetAs%20Takla%20Atma _astakla_atma)
  (Transformation|SetActorLocationAndRotation (Transformation|GetWorldLocation _boat_area) (Transformation|GetWorldRotation _boat_area) false true)
  (Pawn|Possess (Game|GetPlayerController 0) (Variables|Default|GetBP_Ship))
  (Class|PhysicsConstraintComponent|SetConstrainedComponents (Variables|/Game/AFAD/BP_Ship.BP_Ship_C|GetPhysicsConstraint (Variables|Default|GetBP_Ship)) (Variables|/Game/AFAD/BP_Ship.BP_Ship_C|GetShip (Variables|Default|GetBP_Ship)) "None" (Variables|Default|GetPlastic_Boat) "None")
  (Rendering|SetVisibility (Variables|/Game/AFAD/BP_Ship.BP_Ship_C|GetCable (Variables|Default|GetBP_Ship)) true false)
  (bind _asgm_afad (Utilities|Casting|CastToGM_Afad (Game|GetGameMode)))
  (Default|ShipHealthVisibility (Variables|/Game/AFAD/GM_Afad.GM_Afad_C|GetCan _asgm_afad))
  (Default|BoatHealthHidden (Variables|/Game/AFAD/GM_Afad.GM_Afad_C|GetCan _asgm_afad))
  (Utilities|FlowControl|Delay 1.0))

(event Custom|CanAzalt
  (bind _bp_ship (Variables|Default|GetBP_Ship))
  (bind _boat_area (Variables|/Game/AFAD/BP_Ship.BP_Ship_C|GetBoat%20Area _bp_ship))
  (if (not (Variables|Default|GetCanPossess))
    (Variables|Default|SetHealth2 (Math|Float|Clamp(Float) (- (Variables|Default|GetHealth2) 2.0) 0.0 1e+02))
    (if (== (Variables|Default|GetHealth2) 0.0)
      (Transformation|SetActorLocationAndRotation (Transformation|GetWorldLocation _boat_area) (Transformation|GetWorldRotation _boat_area) false true)
      (Pawn|Possess (Game|GetPlayerController 0) (Variables|Default|GetBP_Ship))
      (Class|PhysicsConstraintComponent|SetConstrainedComponents (Variables|/Game/AFAD/BP_Ship.BP_Ship_C|GetPhysicsConstraint (Variables|Default|GetBP_Ship)) (Variables|/Game/AFAD/BP_Ship.BP_Ship_C|GetShip (Variables|Default|GetBP_Ship)) "None" (Variables|Default|GetPlastic_Boat) "None")
      (Rendering|SetVisibility (Variables|/Game/AFAD/BP_Ship.BP_Ship_C|GetCable (Variables|Default|GetBP_Ship)) true false)
      (bind _asgm_afad (Utilities|Casting|CastToGM_Afad (Game|GetGameMode)))
      (Default|ShipHealthVisibility (Variables|/Game/AFAD/GM_Afad.GM_Afad_C|GetCan _asgm_afad))
      (Default|BoatHealthHidden (Variables|/Game/AFAD/GM_Afad.GM_Afad_C|GetCan _asgm_afad))
      (Utilities|FlowControl|Delay 1.0))))

(event Custom|CanArttır
  (Variables|Default|SetHealth2 (Math|Float|Clamp(Float) (+ (Variables|Default|GetHealth2) 1e+02) 0.0 1e+02))
  (if (== (Variables|Default|GetHealth2) 1e+02)
    _))

(event Input|EnhancedActionEvents|EnhancedInputActionIA_Move_Ship
  (params (ActionValue :type Float%20%28double-precision%29) (ElapsedSeconds :type Float%20%28double-precision%29) (TriggeredSeconds :type Float%20%28double-precision%29) (InputAction :type Input%20Action%20Object%20Reference :default "/Game/Input/Actions/IA_Move_Ship.IA_Move_Ship"))
  (Physics|AddForce (Variables|Default|GetPlastic_Boat) (Math|Vector|RotateVector (Math|Vector|MakeVector (* ActionValue 4e+02) 0.0 0.0) (Math|Rotator|CombineRotators (Transformation|GetActorRotation) "0.000000,90.000000,0.000000")) "None" true))

(event Input|EnhancedActionEvents|EnhancedInputActionIA_Steer_Ship
  (params (ActionValue :type Float%20%28double-precision%29) (ElapsedSeconds :type Float%20%28double-precision%29) (TriggeredSeconds :type Float%20%28double-precision%29) (InputAction :type Input%20Action%20Object%20Reference :default "/Game/Input/Actions/IA_Steer_Ship.IA_Steer_Ship"))
  (Class|PrimitiveComponent|AddTorqueinDegrees (Variables|Default|GetPlastic_Boat) (Math|Vector|MakeVector 0.0 0.0 (* ActionValue 5e+01)) "None" true))

(event EventBeginPlay
  (if (<= (Math|Vector|VectorLength (Transformation|GetComponentVelocity (Variables|Default|GetPlastic_Boat))) 1e+01)
    (Utilities|FlowControl|DoOnce false :!label _label
      (:Completed
        (bind _returnvalue (Utilities|Time|SetTimerbyFunctionName 0 "CanAzalt" 1.0 true))))
    (else
      (Utilities|Time|ClearandInvalidateTimerbyHandle _returnvalue)
      (goto _label Reset))))

(event EventPossessed
  (params (NewController :type Controller%20Object%20Reference))
  (bind _asbp_plastic_boat (Utilities|Casting|CastToBP_Plastic_Boat (Game|Player|GetPlayerPawn 0)))
  (Input|AddMappingContext (PlayerController|LocalPlayerSubsystems|GetEnhancedInputLocalPlayerSubsystem (Pawn|GetLocalViewingPlayerController _asbp_plastic_boat)) "/Game/Input/IMC_Plastic_Boat.IMC_Plastic_Boat" 1 "(bIgnoreAllPressedKeysUntilRelease=True,bForceImmediately=False,bNotifyUserSettings=False)")
  (bind _returnvalue (Actor|GetActorOfClass "/Game/AFAD/BP_Ship.BP_Ship_C"))
  (Variables|Default|SetBP_Ship _returnvalue))

(event Input|MouseEvents|MouseX
  (params (AxisValue :type Float%20%28single-precision%29))
  (Pawn|Input|AddControllerYawInput AxisValue))

(event Input|MouseEvents|MouseY
  (params (AxisValue :type Float%20%28single-precision%29))
  (Pawn|Input|AddControllerPitchInput (* AxisValue -1.0)))

(event Input|KeyboardEvents|F
  (params (Key :type Key%20Structure :default "None"))
  (bind _bp_ship (Variables|Default|GetBP_Ship))
  (bind _boat_area (Variables|/Game/AFAD/BP_Ship.BP_Ship_C|GetBoat%20Area _bp_ship))
  (:Pressed
    (if (Variables|Default|GetCanPossess)
      (bind _asgm_afad (Utilities|Casting|CastToGM_Afad (Game|GetGameMode)))
      (Default|ShipHealthVisibility (Variables|/Game/AFAD/GM_Afad.GM_Afad_C|GetCan _asgm_afad))
      (Default|BoatHealthHidden (Variables|/Game/AFAD/GM_Afad.GM_Afad_C|GetCan _asgm_afad))
      (Transformation|SetActorLocationAndRotation (Transformation|GetWorldLocation _boat_area) (Transformation|GetWorldRotation _boat_area) false true)
      (Pawn|Possess (Game|GetPlayerController 0) (Variables|Default|GetBP_Ship))
      (Class|PhysicsConstraintComponent|SetConstrainedComponents (Variables|/Game/AFAD/BP_Ship.BP_Ship_C|GetPhysicsConstraint (Variables|Default|GetBP_Ship)) (Variables|/Game/AFAD/BP_Ship.BP_Ship_C|GetShip (Variables|Default|GetBP_Ship)) "None" (Variables|Default|GetPlastic_Boat) "None")
      (Rendering|SetVisibility (Variables|/Game/AFAD/BP_Ship.BP_Ship_C|GetCable (Variables|Default|GetBP_Ship)) true false)
      (else
        (Development|PrintString "Ship Far")))))

(event Input|KeyboardEvents|E
  (params (Key :type Key%20Structure :default "None"))
  (:Pressed
    (bind _hitactor (Utilities|Interact1)
      (:IsValid
        (Class|BPIInteract1|Interactable1(Message) _hitactor)
        (Audio|PlaySound2D "/Game/AFAD/Sesler/PickUp.PickUp" 1.0 1.0 0.0 0 0)))))

(fn ConstructionScript)

(fn GetInteractState1
  (return false))