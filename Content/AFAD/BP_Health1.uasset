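; BP_Health1 is a health pickup that adds a fixed amount of health to the player's boat.
; Two interaction events each destroy the Health component, then cast the player pawn to BP_Ship or BP_Plastic_Boat to raise that pawn's health variable.
; The health addition has no clamp, and both GetInteractState functions always return false.
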(event EventInteractable1
  (Components|DestroyComponent (Variables|Default|GetHealth))
  (bind _asbp_plastic_boat (Utilities|Casting|CastToBP_Plastic_Boat (Game|Player|GetPlayerPawn 0)))
  (Variables|/Game/AFAD/BP_Plastic_Boat.BP_Plastic_Boat_C|SetHealth2 _asbp_plastic_boat (+ (Variables|/Game/AFAD/BP_Plastic_Boat.BP_Plastic_Boat_C|GetHealth2 _asbp_plastic_boat) 5e+01)))

(event EventInteractable
  (Components|DestroyComponent (Variables|Default|GetHealth))
  (bind _asbp_ship (Utilities|Casting|CastToBP_Ship (Game|Player|GetPlayerPawn 0)))
  (Variables|/Game/AFAD/BP_Ship.BP_Ship_C|SetHealth _asbp_ship (+ (Variables|/Game/AFAD/BP_Ship.BP_Ship_C|GetHealth _asbp_ship) 5e+01)))

(fn ConstructionScript)

(fn GetInteractState
  (return false))

(fn GetInteractState1
  (return false))