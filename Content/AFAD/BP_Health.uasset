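; BP_Health is a health pickup that restores the player's ship when interacted with.
; The Interactable event destroys its own Health component, then casts the player pawn to BP_Ship and adds a fixed amount to its Health, with no clamp.
; Only that component is removed, not the actor, and both GetInteractState functions always return false.
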(event EventInteractable
  (Components|DestroyComponent (Variables|Default|GetHealth))
  (bind _asbp_ship (Utilities|Casting|CastToBP_Ship (Game|Player|GetPlayerPawn 0)))
  (Variables|/Game/AFAD/BP_Ship.BP_Ship_C|SetHealth _asbp_ship (+ (Variables|/Game/AFAD/BP_Ship.BP_Ship_C|GetHealth _asbp_ship) 5e+01)))

(fn ConstructionScript)

(fn GetInteractState
  (return false))

(fn GetInteractState1
  (return false))