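; BP_Kamira is an interactable rescue target with a 15-second countdown, skipped when Safe2 is set.
; Tick writes the remaining timer seconds into the WB_Sayac widget.
; Either interact event stops the timer, flags Kamira on BP_İskele and calls SetKamiraCaught on the GM_Afad WBKayıp widget.
; Timeout calls DiscardKamira instead; both outcomes hide the countdown and destroy the Kamira and HelpWoman components.
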(event Custom|TimeOut
  (Rendering|SetVisibility (Variables|Default|GetWidget) false false)
  (bind _asgm_afad (Utilities|Casting|CastToGM_Afad (Game|GetGameMode)))
  (Default|DiscardKamira (Variables|/Game/AFAD/GM_Afad.GM_Afad_C|GetWB_Kayıp _asgm_afad))
  (Components|DestroyComponent (Variables|Default|GetKamira))
  (Components|DestroyComponent (Variables|Default|GetHelpWoman)))

(event EventBeginPlay
  (if (Variables|Default|GetSafe2)
    (Components|DestroyComponent (Variables|Default|GetWidget))
    (else
      (bind _returnvalue (Utilities|Time|SetTimerbyEvent (delegate Custom|TimeOut) 15.0))
      (Variables|Default|SetKamiraTimerHandle _returnvalue))))

(event EventTick
  (params (DeltaSeconds :type Float%20%28single-precision%29))
  (Utilities|FlowControl|Delay 0.1)
  (Utilities|IsValid (Variables|Default|GetWidget)
    (:Is%20Valid
      (bind _aswb_sayac (Utilities|Casting|CastToWB_Sayac (UserInterface|GetUserWidgetObject (Variables|Default|GetWidget))))
      (Rendering|Components|TextRender|SetText (Variables|/Game/AFAD/WB_Sayac.WB_Sayac_C|GetSayacText _aswb_sayac) (Utilities|Text|ToText(Integer) (Math|Float|Round (Utilities|Time|GetTimerRemainingTimebyHandle (Variables|Default|GetKamiraTimerHandle))))))))

(event EventInteractable
  (Utilities|Time|ClearandInvalidateTimerbyHandle (Variables|Default|GetKamiraTimerHandle))
  (Rendering|SetVisibility (Variables|Default|GetWidget) false false)
  (bind _returnvalue (Actor|GetActorOfClass "/Game/AFAD/BP_İskele.BP_İskele_C"))
  (Variables|/Game/AFAD/BP_İskele.BP_İskele_C|SetKamira _returnvalue true)
  (Components|DestroyComponent (Variables|Default|GetKamira))
  (bind _asgm_afad (Utilities|Casting|CastToGM_Afad (Game|GetGameMode)))
  (Default|SetKamiraCaught (Variables|/Game/AFAD/GM_Afad.GM_Afad_C|GetWB_Kayıp _asgm_afad))
  (Components|DestroyComponent (Variables|Default|GetHelpWoman)))

(event EventInteractable1
  (Utilities|Time|ClearandInvalidateTimerbyHandle (Variables|Default|GetKamiraTimerHandle))
  (Rendering|SetVisibility (Variables|Default|GetWidget) false false)
  (bind _returnvalue (Actor|GetActorOfClass "/Game/AFAD/BP_İskele.BP_İskele_C"))
  (Variables|/Game/AFAD/BP_İskele.BP_İskele_C|SetKamira _returnvalue true)
  (Components|DestroyComponent (Variables|Default|GetKamira))
  (bind _asgm_afad (Utilities|Casting|CastToGM_Afad (Game|GetGameMode)))
  (Default|SetKamiraCaught (Variables|/Game/AFAD/GM_Afad.GM_Afad_C|GetWB_Kayıp _asgm_afad))
  (Components|DestroyComponent (Variables|Default|GetHelpWoman)))

(fn ConstructionScript)

(fn GetInteractState
  (return false))

(fn GetInteractState1
  (return false))