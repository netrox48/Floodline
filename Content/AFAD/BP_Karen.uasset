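; BP_Karen is an interactable Karen in the AFAD game that is marked as caught when interacted with.
; Two matching interact events each destroy the Karen component, then call SetKarenCaught on the WBKayıp widget held by GM_Afad.
; Both GetInteractState functions always return false.
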(event EventInteractable
  (Components|DestroyComponent (Variables|Default|GetKaren))
  (bind _asgm_afad (Utilities|Casting|CastToGM_Afad (Game|GetGameMode)))
  (Default|SetKarenCaught (Variables|/Game/AFAD/GM_Afad.GM_Afad_C|GetWB_Kayıp _asgm_afad)))

(event EventInteractable1
  (Components|DestroyComponent (Variables|Default|GetKaren))
  (bind _asgm_afad (Utilities|Casting|CastToGM_Afad (Game|GetGameMode)))
  (Default|SetKarenCaught (Variables|/Game/AFAD/GM_Afad.GM_Afad_C|GetWB_Kayıp _asgm_afad)))

(fn ConstructionScript)

(fn GetInteractState
  (return false))

(fn GetInteractState1
  (return false))