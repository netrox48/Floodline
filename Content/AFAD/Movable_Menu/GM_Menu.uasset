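; GM_Menu, by its name the menu game mode, brings up the menu screens and their sound on BeginPlay.
; A Sequence adds WB_Menu to the viewport, starts a 12-second delay, and plays the Waves sound without waiting for it.
; After the delay it adds WB_Menu1 without removing the first widget, then shows the mouse cursor.
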(event EventBeginPlay
  (Utilities|FlowControl|Sequence
    (:then_0
      (bind _returnvalue (UserInterface|CreateWidget "/Game/AFAD/Movable_Menu/WB_Menu.WB_Menu_C" (Game|GetPlayerController 0)))
      (bind _output_get (Variables|Default|SetMainMenuWidget _returnvalue))
      (UserInterface|Viewport|AddtoViewport _output_get 0)
      (Utilities|FlowControl|Delay 12.0)
      (bind _returnvalue_2 (UserInterface|CreateWidget "/Game/AFAD/Movable_Menu/WB_Menu1.WB_Menu1_C" (Game|GetPlayerController 0)))
      (bind _output_get_2 (Variables|Default|SetMainMenuWidget1 _returnvalue_2))
      (UserInterface|Viewport|AddtoViewport _output_get_2 0)
      (Variables|/Script/Engine.PlayerController|SetbShowMouseCursor (Game|GetPlayerController 0) true))
    (:then_1
      (Audio|PlaySound2D "/Game/AFAD/Sesler/Waves.Waves" 1.0 1.0 0.0 0 0))))

(fn ConstructionScript)